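; BP_PE_EnemyBase is the enemy base Blueprint for Project Entropy, showing the enemy's current and maximum AP on a text render.
; On BeginPlay it binds UpdateAPText to the StatComponent's AP-changed event and calls it once with the starting values.
; Later updates are event-driven, writing the text as current/max, with Tick and overlap left unused.
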(event Custom|Update%20AP%20Text
  (params (CurrentAP :type Integer) (MaxAP :type Integer) (Delta :type Integer))
  (Rendering|Components|TextRender|SetText (Variables|Default|GetTextRender) (Utilities|Text|ToText(String) (Utilities|String|Append (Utilities|String|ToString(Integer) CurrentAP) "/" (Utilities|String|ToString(Integer) MaxAP)))))

(event EventBeginPlay
  (bind _statcomponent (Variables|Default|GetStatComponent))
  (EventDispatchers|BindEventtoOnAPChanged _statcomponent (delegate Custom|Update%20AP%20Text))
  (CallFunction|UpdateAPText (Variables|/Script/Project_Entropy.ACStatComponent|GetCurrentAP _statcomponent) (Variables|/Script/Project_Entropy.ACStatComponent|GetMaxAP _statcomponent)))

(event Collision|EventActorBeginOverlap
  (params (OtherActor :type Actor%20Object%20Reference)))

(event EventTick
  (params (DeltaSeconds :type Float%20%28single-precision%29)))

(fn ConstructionScript)