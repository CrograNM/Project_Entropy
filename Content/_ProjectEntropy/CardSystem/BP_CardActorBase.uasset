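; Base 3D card actor for the card system that shows rarity through a mesh material looked up in the global card theme.
; Casting-ready animation chains timelines: lerp to a middle transform, then to a final one with a full yaw spin.
; It then notifies the player controller's card interaction component and starts a sine-based idle wobble on the mesh, which cancelling stops.
; Hovering during casting nudges the mesh along X via a reversible timeline.
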(event EventBeginPlay)

(event Collision|EventActorBeginOverlap
  (params (OtherActor :type Actor%20Object%20Reference)))

(event EventTick
  (params (DeltaSeconds :type Float%20%28single-precision%29)))

(event EventPlayCastingReadyAnimation
  (bind _middletransform (Variables|Default|GetMiddleTransform))
  (bind _fianltransform (Variables|Default|GetFianlTransform))
  ;[0.15 0.15 0.15 0.5] Play Casting Ready Anim
  (Variables|Default|SetStartTransform (Transformation|GetRelativeTransform (Variables|Default|GetRootScene)))
  (bind _alpha (Timeline|TL_MoveToMiddle PlayFromStart)
    (:Update
      (Transformation|SetActorRelativeTransform (Math|Transform|Lerp(Transform) (Variables|Default|GetStartTransform) (Variables|Default|GetMiddleTransform) _alpha) false false))
    (:Finished
      ;;[0.15 0.15 0.15 0.5] Spin
      (Variables|Default|SetRandomSpinTarget (Math|Rotator|MakeRotator 0.0 0.0 3.6e+02))
      (bind _alpha_2 (Timeline|TL_MoveToFinal PlayFromStart)
        (:Update
          (Transformation|SetActorRelativeTransform (Math|Transform|MakeTransform (Math|Vector|Lerp(Vector) (.location _middletransform) (.location _fianltransform) _alpha_2) (Math|Rotator|CombineRotators (Math|Rotator|MakeRotator (* _alpha_2 (.roll (Variables|Default|GetRandomSpinTarget))) (* _alpha_2 (.pitch (Variables|Default|GetRandomSpinTarget))) (* _alpha_2 (.yaw (Variables|Default|GetRandomSpinTarget)))) (Math|Rotator|Lerp(Rotator) (.rotation _middletransform) (.rotation _fianltransform) _alpha_2 true))) false false))
        (:Finished
          ;;[0.15 0.15 0.15 0.5] Finish -> Idle
          (bind _aspe_player_controller (Utilities|Casting|CastToPE_PlayerController (Game|GetPlayerController 0)))
          (Class|ACCardInteractionComponent|OnCastingReadyFinished (Variables|/Script/Project_Entropy.PE_PlayerController|GetCardInteractionComp _aspe_player_controller))
          (Variables|Default|SetCardMesh%20Relative%20Loc%20Saved (Variables|/Script/Engine.SceneComponent|GetRelativeLocation (Variables|Default|GetCardMesh)))
          (bind _timealpha (Timeline|TL_IdleFloating PlayFromStart)
            (:Update
              (Transformation|SetRelativeRotation (Variables|Default|GetCardMesh) (Math|Rotator|CombineRotators (Math|Rotator|MakeRotator (* (Math|Trig|Sin(Degrees) _timealpha) 4.0) (* (Math|Trig|Sin(Degrees) _timealpha) 3.0) (* (Math|Trig|Cos(Degrees) _timealpha) -5.0)) (.rotation (Variables|Default|GetFianlTransform))) false false))))))))

(event EventPlayCancelCastingAnimation
  (params (ReturnHandTransform :type Transform))
  ;[0.15 0.15 0.15 0.5] Play Casting Ready Anim
  ;;[0.15 0.15 0.15 0.5] Finish -> Idle
  (bind _timealpha (Timeline|TL_IdleFloating Stop)
    (:Update
      (Transformation|SetRelativeRotation (Variables|Default|GetCardMesh) (Math|Rotator|CombineRotators (Math|Rotator|MakeRotator (* (Math|Trig|Sin(Degrees) _timealpha) 4.0) (* (Math|Trig|Sin(Degrees) _timealpha) 3.0) (* (Math|Trig|Cos(Degrees) _timealpha) -5.0)) (.rotation (Variables|Default|GetFianlTransform))) false false))))

(event EventOnCastingHoverStateChanged
  (params (IsHovered :type Boolean))
  (bind _cardmesh_relative_loc_saved (Variables|Default|GetCardMesh%20Relative%20Loc%20Saved))
  ;[0.15 0.15 0.15 0.5] Casting Card Hovering
  (if IsHovered
    (bind _alpha (Timeline|TL_IdleHoveringWhenCasted PlayFromStart)
      (:Update
        (Transformation|SetRelativeLocation (Variables|Default|GetCardMesh) (Math|Vector|Lerp(Vector) _cardmesh_relative_loc_saved (+ _cardmesh_relative_loc_saved "5.000000,0.000000,0.000000") _alpha) false false)))
    (else
      (Timeline|TL_IdleHoveringWhenCasted ReverseFromEnd))))

(event EventInitializeCardVisual
  (params (InCardInstance :type PE%20Card%20Instance%20Object%20Reference))
  (bind _returnvalue (Class|PECardInstance|GetBaseCardData InCardInstance))
  (bind _globalcardtheme (Variables|Default|GetGlobalCardTheme))
  (bind _rarity (Variables|/Script/Project_Entropy.PE_CardData|GetRarity _returnvalue))
  (bind _raritymaterialmap (Variables|/Script/Project_Entropy.PE_CardThemeData|GetRarityMaterialMap _globalcardtheme))
  (bind (_value _returnvalue_2) (Utilities|Map|Find _raritymaterialmap _rarity))
  ;[0.15 0.15 0.15 0.5] Initialize Card Visual
  (if _returnvalue_2
    (Rendering|Material|SetMaterial (Variables|Default|GetCardMesh) 0 _value)
    (else
      (Development|PrintString "CardActor: Rarity Material Map - Find Failed"))))

(fn ConstructionScript)