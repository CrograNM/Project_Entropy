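; Player controller for Project Entropy that manages UI widgets and debug key bindings.
; P toggles the pause menu with cursor and input-mode switching, sharing the close path with CloseWidget.
; SetBattleUIVisibility creates or removes a local battle test widget, and ShowToastMessage spawns toast popups.
; Test keys trigger card draws, toggle grid movement, and flip between Base and Battle input modes; BeginPlay does nothing, leaving older setup logic disconnected.
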(event Custom|CloseWidget
  ;[0.15 0.15 0.15 0.5] Pause Menu
  (Variables|Default|GetActive%20Widget
    (:then
      (Widget|RemovefromParent (Variables|Default|GetActive%20Widget))
      (Variables|Default|SetActive%20Widget 0)
      (Input|SetInputModeGameOnly self false)
      (Variables|Default|SetbShowMouseCursor false))
    (:else)))

(event EventBeginPlay)

(event EventSetBattleUIVisibility
  (params (bVisible :type Boolean))
  (if (and bVisible (Pawn|IsLocalPlayerController))
    (Variables|Default|GetBattle%20Widget
      (:then)
      (:else
        (bind _returnvalue (UserInterface|CreateWidget "/Game/_ProjectEntropy/UI/WBP_BattleTest.WBP_BattleTest_C" self))
        (bind _output_get (Variables|Default|SetBattle%20Widget _returnvalue))
        (UserInterface|Viewport|AddtoViewport _output_get 0)))
    (else
      (Variables|Default|GetBattle%20Widget
        (:then
          (Widget|RemovefromParent (Variables|Default|GetBattle%20Widget))
          (Variables|Default|SetBattle%20Widget 0))
        (:else)))))

(event EventShowToastMessage
  (params (Message :type Text%20%28by%20ref%29))
  ;[0.15 0.15 0.15 0.5] Show Toast Message
  (bind _returnvalue (UserInterface|CreateWidget "/Game/_ProjectEntropy/UI/WBP_ToastMessage.WBP_ToastMessage_C"))
  (Rendering|Components|TextRender|SetText (Variables|/Game/_ProjectEntropy/UI/WBP_ToastMessage.WBP_ToastMessage_C|GetText_ToastMessage _returnvalue) Message)
  (UserInterface|Viewport|AddtoViewport _returnvalue 0))

(event Input|KeyboardEvents|P
  (params (Key :type Key%20Structure :default "None"))
  ;[0.15 0.15 0.15 0.5] Pause Menu
  (:Pressed
    (Variables|Default|GetActive%20Widget
      (:then
        (Variables|Default|GetActive%20Widget
          (:then
            (Widget|RemovefromParent (Variables|Default|GetActive%20Widget))
            (Variables|Default|SetActive%20Widget 0)
            (Input|SetInputModeGameOnly self false)
            (Variables|Default|SetbShowMouseCursor false))
          (:else)))
      (:else
        (bind _returnvalue (UserInterface|CreateWidget "/Game/_ProjectEntropy/UI/Menu/WBP_PauseMenu.WBP_PauseMenu_C" self))
        (bind _output_get (Variables|Default|SetActive%20Widget _returnvalue))
        (UserInterface|Viewport|AddtoViewport _output_get 0)
        (Input|SetInputModeGameandUI self 0 "DoNotLock" true false)
        (Variables|Default|SetbShowMouseCursor true)))))

(event Input|KeyboardEvents|I
  (params (Key :type Key%20Structure :default "None"))
  (:Pressed
    (Utilities|FlowControl|FlipFlop
      (:A
        ;[0.15 0.15 0.15 0.5] Switch Input Mode
        (Class|PEPlayerController|SwitchInputMode "Base")
        (Development|PrintString "Input Mode: Base"))
      (:B
        (Class|PEPlayerController|SwitchInputMode "Battle")
        (Development|PrintString "Input Mode: Battle")))))

(event Input|KeyboardEvents|M
  (params (Key :type Key%20Structure :default "None"))
  ;[0.15 0.15 0.15 0.5] Toggle Movement
  (:Pressed
    (Class|PEPlayerController|ToggleGridMovementActivation)
    (Development|PrintString "Movement Mode Toggled")))

(event Input|KeyboardEvents|SpaceBar
  (params (Key :type Key%20Structure :default "None"))
  ;[0.15 0.15 0.15 0.5] Draw Test
  (:Pressed
    (Class|PEPlayerController|OnTestDrawCard 10)))

(fn ConstructionScript)